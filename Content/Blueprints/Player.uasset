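; Player Blueprint that fires an equipped gun component and cycles between rifle, shotgun and rocket launcher.
; Fire input calls Shoot on the current Gun, initially the rifle; weapon switching destroys that component and adds the next, printing the selection for debug.
; The construction script writes the PlaneMesh world position into the Cutoff material parameter collection.
; Tick's movement and boundary update calls are disabled, so that position is not refreshed per frame here.
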(event EventBeginPlay
  (Variables|Default|SetGun (Variables|Default|GetGun_Rifle)))

(event Collision|EventActorBeginOverlap
  (params (OtherActor :type Actor%20Object%20Reference)))

(event EventTick
  (params (DeltaSeconds :type Float%20%28single-precision%29))
  (CallFunction|MovementTick "0, 0, 0" "0, 0, 0" DeltaSeconds)
  (CallFunction|UpdateBoundryCheck))

(event Input|ActionEvents|InputActionFirePrimary
  (params (Key :type Key%20Structure))
  (:Pressed
    (Default|Shoot (Variables|Default|GetGun) self)))

(event Input|ActionEvents|InputActionChangeMainWeapon
  (params (Key :type Key%20Structure))
  ;[1 1 1] Swap Gun
  (:Pressed
    ;;[1 1 1] Remove old gun
    (Components|DestroyComponent (Variables|Default|GetGun))
    (bind _output_get (Variables|Default|SetEquipedGun (Math|Integer|%(Integer) (+ (Variables|Default|GetEquipedGun) 1) 3)))
    (switch int _output_get
      (:Default
        (Development|PrintString "!!!INVALID GUN!!!"))
      (:0
        (bind _returnvalue (AddComponent|AddGunRifle))
        (Variables|Default|SetGun _returnvalue)
        ;;[1 1 1] Debug print statement
        (Development|PrintString (Utilities|String|Append "Now using gun:" (Utilities|String|ToString(Integer) (Variables|Default|GetEquipedGun))) :!label _label))
      (:1
        (bind _returnvalue_2 (AddComponent|AddGunShotgun))
        (Variables|Default|SetGun _returnvalue_2)
        (goto _label))
      (:2
        (bind _returnvalue_3 (AddComponent|AddGunRocketLauncher))
        (Variables|Default|SetGun _returnvalue_3)
        (goto _label)))))

(fn ConstructionScript
  (|CallParentFunction)
  (Rendering|Material|SetVectorParameterValue "/Game/Blueprints/Cutoff_Collection.Cutoff_Collection" "Position" (Math|Conversions|ToLinearColor(Vector) (Transformation|GetWorldLocation (Variables|Default|GetPlane%20mesh))) :!class /Script/Engine.KismetMaterialLibrary))

(fn UpdateBoundryCheck
  (Rendering|Material|SetVectorParameterValue "/Game/Blueprints/Cutoff_Collection.Cutoff_Collection" "Position" (Math|Conversions|ToLinearColor(Vector) (Transformation|GetWorldLocation (Variables|Default|GetPlane%20mesh))) :!class /Script/Engine.KismetMaterialLibrary))