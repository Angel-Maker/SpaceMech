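; PlayerMech is the player-controlled flying mech, which turns input into movement and fires swappable guns.
; Each Tick it writes axis input to thrust and rotation variables before calling the parent, and feeds the ship's position to the Cutoff material parameter collection.
; Switching weapons destroys the gun component and adds the next of rifle, shotgun or rocket launcher.
; The T key runs a repeated-fire test.
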(event EventBeginPlay
  (|CallParentFunction)
  (Variables|Default|SetLookRate 5e+01) ; This should be a setting editable by user and assigned by higher level systems
  ;[1 1 1] Set starting gun
  (bind _returnvalue (AddComponent|AddGunRifle))
  (Variables|Default|SetGun _returnvalue))

(event Collision|EventActorBeginOverlap
  (params (OtherActor :type Actor%20Object%20Reference))
  (|CallParentFunction OtherActor) ; This node is disabled and will not be called.\nDrag off pins to build functionality.
)

(event EventTick
  (params (DeltaSeconds :type Float%20%28single-precision%29))
  (CallFunction|MovementInput)
  (CallFunction|UpdateBoundaryCheck)
  (|CallParentFunction DeltaSeconds))

(event Input|ActionEvents|InputActionFirePrimary
  (params (Key :type Key%20Structure :default "None"))
  (:Pressed
    (Default|Shoot (Variables|Default|GetGun) self)))

(event Input|ActionEvents|InputActionChangeMainWeapon
  (params (Key :type Key%20Structure :default "None"))
  ;[1 1 1] Swap Gun
  (:Pressed
    ;;[1 1 1] Remove old gun
    (Components|DestroyComponent (Variables|Default|GetGun))
    (bind _output_get (Variables|Default|SetEquipedGun (Math|Integer|%(Integer) (+ (Variables|Default|GetEquipedGun) 1) 3)))
    (switch int _output_get
      (:Default
        (Development|PrintString "!!!INVALID GUN!!!"))
      (:0
        (bind _returnvalue (AddComponent|AddGunRifle))
        (Variables|Default|SetGun _returnvalue)
        ;;[1 1 1] Debug print statement
        (Development|PrintString (Utilities|String|Append "Now using gun:" (Utilities|String|ToString(Integer) (Variables|Default|GetEquipedGun))) :!label _label))
      (:1
        (bind _returnvalue_2 (AddComponent|AddGunShotgun))
        (Variables|Default|SetGun _returnvalue_2)
        (goto _label))
      (:2
        (bind _returnvalue_3 (AddComponent|AddGunRocketLauncher))
        (Variables|Default|SetGun _returnvalue_3)
        (goto _label)))))

(event Input|KeyboardEvents|T
  (params (Key :type Key%20Structure :default "None"))
  ;[1 1 1] Test code
  (:Pressed
    (Utilities|ForLoopwithDelay 1 100 0.1
      (:LoopBody
        (Default|Shoot (Variables|Default|GetGun) self))
      (:Completed
        (Utilities|FlowControl|Delay 5.0)
        (Development|PrintString "Check Frames")))))

(fn ConstructionScript
  (|CallParentFunction))

(fn UpdateBoundaryCheck
  (Rendering|Material|SetVectorParameterValue "/Game/Assets/AreaBarrier/Cutoff_Collection.Cutoff_Collection" "Position" (Math|Conversions|ToLinearColor(Vector) (Transformation|GetWorldLocation (Variables|Default|GetSMShip))) :!class /Script/Engine.KismetMaterialLibrary))

(fn MovementInput
  (Variables|Default|SetThrustInput (Math|Vector|MakeVector (Input|AxisValues|GetMoveForward) (Input|AxisValues|GetMoveRight) (Input|AxisValues|GetMoveUp)))
  (Variables|Default|SetRotationInput (Math|Rotator|MakeRotator 0.0 (Input|AxisValues|GetLookUp) (Input|AxisValues|GetLookRight))))