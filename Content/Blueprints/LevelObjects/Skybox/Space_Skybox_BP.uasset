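; Space skybox actor that applies a configurable material and brightness settings to its sky mesh.
; It writes star brightness, power and scene brightness variables into the Skybox_Params material parameter collection, then sets the chosen material on the static mesh.
; The same logic runs in the construction script for editor preview and again on BeginPlay for runtime.
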(event EventBeginPlay
  ;[1 1 1] Sets the value at runtime
  (Rendering|Material|SetScalarParameterValue "/Game/Blueprints/LevelObjects/Skybox/Skybox_Params.Skybox_Params" "Star_Brightness" (Variables|Default|GetStar_Brightness) :!class /Script/Engine.KismetMaterialLibrary)
  (Rendering|Material|SetScalarParameterValue "/Game/Blueprints/LevelObjects/Skybox/Skybox_Params.Skybox_Params" "Power" (Variables|Default|GetPower) :!class /Script/Engine.KismetMaterialLibrary)
  (Rendering|Material|SetScalarParameterValue "/Game/Blueprints/LevelObjects/Skybox/Skybox_Params.Skybox_Params" "Scene_Brightness" (Variables|Default|GetScene_Brightness) :!class /Script/Engine.KismetMaterialLibrary)
  (Rendering|Material|SetMaterial (Variables|Default|GetStaticMesh) 0 (Variables|Default|Getmarerial)))

(event Collision|EventActorBeginOverlap
  (params (OtherActor :type Actor%20Object%20Reference)))

(event EventTick
  (params (DeltaSeconds :type Float%20%28single-precision%29)))

(fn ConstructionScript
  ;[1 1 1] Sets the values for editor
  (Rendering|Material|SetScalarParameterValue "/Game/Blueprints/LevelObjects/Skybox/Skybox_Params.Skybox_Params" "Star_Brightness" (Variables|Default|GetStar_Brightness) :!class /Script/Engine.KismetMaterialLibrary)
  (Rendering|Material|SetScalarParameterValue "/Game/Blueprints/LevelObjects/Skybox/Skybox_Params.Skybox_Params" "Power" (Variables|Default|GetPower) :!class /Script/Engine.KismetMaterialLibrary)
  (Rendering|Material|SetScalarParameterValue "/Game/Blueprints/LevelObjects/Skybox/Skybox_Params.Skybox_Params" "Scene_Brightness" (Variables|Default|GetScene_Brightness) :!class /Script/Engine.KismetMaterialLibrary)
  (Rendering|Material|SetMaterial (Variables|Default|GetStaticMesh) 0 (Variables|Default|Getmarerial)))