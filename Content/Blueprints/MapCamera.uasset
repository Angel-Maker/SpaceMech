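; RTS-style map camera pawn with WASD panning, drag-box unit selection and right-click move orders, showing the cursor while possessed.
; Tick pans by a fixed per-frame step and, during left-drag, box-traces between mouse-ray hit points to fill SelectedUnits.
; Selected static mesh actors get a highlight material, reset on the next click.
; Right-click teleports selected actors to the clicked point and shows a marker for one second.
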(event EventBeginPlay
  (bind _returnvalue (AddComponent|AddGameplayTasksComponent))
  (Variables|Default|SetGameplay%20Task%20Component _returnvalue))

(event Collision|EventActorBeginOverlap
  (params (OtherActor :type Actor%20Object%20Reference)))

(event EventTick
  (params (DeltaSeconds :type Float%20%28single-precision%29))
  (bind _self self)
  (bind _returnvalue (Transformation|GetActorLocation _self))
  (bind (_x _y _z) (Math|Vector|BreakVector _returnvalue))
  ;[1 1 1] Change Camera Actor
  (Utilities|FlowControl|Sequence
    (:then_0
      ;;[1 1 1] Update Map Location
      (Transformation|SetActorLocation _self (Math|Vector|MakeVector (+ (Variables|Default|GetUp) _x) (+ _y (Variables|Default|Getright)) _z) true false))
    (:then_1
      ;;[1 1 1] Click and Drag Action
      (if (Variables|Default|GetDragMode)
        (bind _clicklocation (CallFunction|FindClickonPlane))
        (bind (_center _halfsize) (CallFunction|FindDragArea (Variables|Default|GetClickStartPosition) _clicklocation))
        (bind _outhits (Class|KismetSystemLibrary|BoxTraceMulti (Math|Vector|MakeVector (.x _center) (.y _center) (Variables|Default|GetMaxDistance)) (Math|Vector|MakeVector (.x _center) (.y _center) (* -1 (Variables|Default|GetMaxDistance))) _halfsize "0, 0, 0" "TraceTypeQuery4" false 0 "ForDuration" true))
        (bind _output_get (Variables|Default|SetSelectedUnits _outhits))
        (for _array_element _output_get
          (bind _asstatic_mesh_actor (Utilities|Casting|CastToStaticMeshActor (.HitActor (Collision|BreakHitResult _array_element))))
          (Rendering|Material|SetMaterial (Variables|/Script/Engine.StaticMeshActor|GetStaticMeshComponent _asstatic_mesh_actor) 0 "/Game/Assets/Materials/YellowBlaster.YellowBlaster"))))))

(event EventPossessed
  (params (NewController :type Controller%20Object%20Reference))
  (bind _returnvalue (Game|GetPlayerController 0))
  ;[1 1 1] Toggle Mouse Visibility
  (if (!= _returnvalue 0)
    (Variables|/Script/Engine.PlayerController|SetbShowMouseCursor _returnvalue true)))

(event EventUnpossessed
  (params (OldController :type Controller%20Object%20Reference))
  (bind _returnvalue (Game|GetPlayerController 0))
  ;[1 1 1] Toggle Mouse Visibility
  (if (!= _returnvalue 0)
    (Variables|/Script/Engine.PlayerController|SetbShowMouseCursor _returnvalue false)))

(event Input|MouseEvents|LeftMouseButton
  (params (Key :type Key%20Structure))
  ;[1 1 1] Click and Drag Selector
  (:Pressed
    (Variables|Default|SetDragMode true)
    (for _array_element (Variables|Default|GetSelectedUnits)
      (bind _asstatic_mesh_actor (Utilities|Casting|CastToStaticMeshActor (|CollapseGraph_0 _array_element)))
      (Rendering|Material|SetMaterial (Variables|/Script/Engine.StaticMeshActor|GetStaticMeshComponent _asstatic_mesh_actor) 0 "/Game/Assets/UFO/BaseMaterial.BaseMaterial"))
    (Variables|Default|SetSelectedUnits (Utilities|Array|MakeArray ""))
    (bind _clicklocation (CallFunction|FindClickonPlane))
    (Variables|Default|SetClickStartPosition (Math|Vector|MakeVector (.X (Math|Vector|BreakVector _clicklocation)) (.Y (Math|Vector|BreakVector _clicklocation)) (Variables|Default|GetMaxDistance))))
  (:Released
    (Variables|Default|SetDragMode false)))

(event Input|MouseEvents|RightMouseButton
  (params (Key :type Key%20Structure))
  ;[1 1 1] Move Command
  (:Pressed
    (bind _clicklocation (CallFunction|FindClickonPlane))
    (bind _returnvalue (Game|SpawnActorfromClass "/Game/Blueprints/SelectionActor.SelectionActor_C" (Math|Conversions|ToTransform(Vector) _clicklocation) "AlwaysSpawn" 0 0))
    (GameplayTasks|TaskWaitDelay (Variables|Default|GetGameplay%20Task%20Component) 1.0
      (:then
        (for _array_element (Variables|Default|GetSelectedUnits)
          (Transformation|SetActorLocation (|CollapseGraph_0_2 _array_element) _clicklocation false false)))
      (:OnFinish
        (Actor|DestroyActor _returnvalue)))))

(event Input|KeyboardEvents|A
  (params (Key :type Key%20Structure))
  ;[1 1 1] Movement
  (:Pressed
    (Variables|Default|Setright (* (Variables|Default|GetMapMovementSpeed) -1.0)))
  (:Released
    (Variables|Default|Setright 0.0)))

(event Input|KeyboardEvents|S
  (params (Key :type Key%20Structure))
  ;[1 1 1] Movement
  (:Pressed
    (Variables|Default|SetUp (* (Variables|Default|GetMapMovementSpeed) -1.0)))
  (:Released
    (Variables|Default|SetUp 0.0)))

(event Input|KeyboardEvents|W
  (params (Key :type Key%20Structure))
  ;[1 1 1] Movement
  (:Pressed
    (Variables|Default|SetUp (Variables|Default|GetMapMovementSpeed)))
  (:Released
    (Variables|Default|SetUp 0.0)))

(event Input|KeyboardEvents|D
  (params (Key :type Key%20Structure))
  ;[1 1 1] Movement
  (:Pressed
    (Variables|Default|Setright (Variables|Default|GetMapMovementSpeed)))
  (:Released
    (Variables|Default|Setright 0.0)))

(fn ConstructionScript)

(fn FindClickonPlane
  (bind _camera (Variables|Default|GetCamera))
  (bind _returnvalue (Transformation|GetWorldLocation _camera))
  (bind _outhit (Collision|LineTraceByChannel _returnvalue (+ _returnvalue (* (.WorldDirection (Game|Player|ConvertMouseLocationToWorldSpace (Game|GetPlayerController 0))) (Variables|Default|GetMaxMapClickDistance))) "TraceTypeQuery3" false 0 "ForDuration" true "(R=1.000000,G=0.000000,B=0.000000,A=1.000000)" "(R=0.000000,G=1.000000,B=0.000000,A=1.000000)" 2.0))
  (return (.Location (Collision|BreakHitResult _outhit))))

(fn FindDragArea
  (params (Start :type Vector) (End :type Vector))
  (bind _returnvalue (- Start End))
  (bind _returnvalue_2 (+ Start End))
  (bind _returnvalue_3 (/ _returnvalue_2 2.0))
  (bind _returnvalue_4 (/ _returnvalue 2.0))
  (bind (_x _y) (Math|Vector|BreakVector _returnvalue_3))
  (return (Math|Vector2D|MakeVector2D _x _y) (Math|Vector|MakeVector (Math|Float|Absolute(Float) (.x _returnvalue_4)) (Math|Float|Absolute(Float) (.y _returnvalue_4)) 1e+02)))