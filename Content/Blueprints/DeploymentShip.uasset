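; Deployment ship actor that spawns AI mechs for team 1 while that team has tickets left.
; On BeginPlay it finds the GameManager and starts a delayed while loop that checks Team1Tickets.
; Each pass waits briefly, spawns an AIMech at a randomly rotated SpawnRadius offset from PlaneMesh, then reports it through the GameManager's NewMechAdded.
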(event Custom|SpawnMechs
  (bind _gamemanager (Variables|Default|GetGameManager))
  ;[1 1 1] Spawns mechs until tickets are depleated
  (Utilities|WhileLoopwithDelay (> (Variables|/Game/Blueprints/GameManager.GameManager_C|GetTeam1Tickets _gamemanager) 0) 2.0
    (:LoopBody
      (Utilities|FlowControl|Delay 1.0)
      (Game|SpawnActorfromClass "/Game/Blueprints/AIMech.AIMech_C" (Math|Transform|MakeTransform (+ (Math|Vector|RotateVector (Math|Vector|MakeVector (Variables|Default|GetSpawnRadius) 0.0 0.0) (Math|Random|RandomRotator false)) (Transformation|GetWorldLocation (Variables|Default|GetPlane%20mesh)))) "AlwaysSpawn" 0 0)
      (Default|NewMechAdded _gamemanager))))

(event EventBeginPlay
  (|CallParentFunction)
  (bind _returnvalue (Actor|GetActorOfClass "/Game/Blueprints/GameManager.GameManager_C"))
  (Variables|Default|SetGameManager _returnvalue)
  (CallFunction|SpawnMechs))

(event Collision|EventActorBeginOverlap
  (params (OtherActor :type Actor%20Object%20Reference))
  (|CallParentFunction OtherActor) ; This node is disabled and will not be called.\nDrag off pins to build functionality.
)

(event EventTick
  (params (DeltaSeconds :type Float%20%28single-precision%29))
  (|CallParentFunction DeltaSeconds) ; This node is disabled and will not be called.\nDrag off pins to build functionality.
)

(fn ConstructionScript
  (|CallParentFunction))