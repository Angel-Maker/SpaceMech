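; Shotgun weapon Blueprint that fires a spread of bullet actors each time Shoot is called.
; Shoot loops NumberOfBullets times, spawning Bullet 100 units along the local X axis of the passed SpawningActor.
; Each bullet combines that actor's rotation with random pitch and yaw offsets scaled by Accuracy, so higher values widen the spread.
; BeginPlay only calls the parent, and Tick is disabled.
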(event EventBeginPlay
  (|CallParentFunction))

(event EventTick
  (params (DeltaSeconds :type Float%20%28single-precision%29))
  (|CallParentFunction DeltaSeconds) ; This node is disabled and will not be called.\nDrag off pins to build functionality.
)

(event EventShoot
  (params (SpawningActor :type Actor%20Object%20Reference))
  (bind _returnvalue (Transformation|GetActorTransform SpawningActor))
  (bind _accuracy (Variables|Default|GetAccuracy))
  (bind (_location _rotation _scale) (Math|Transform|BreakTransform _returnvalue))
  (for _index (range 1 (Variables|Default|GetNumber_of_bullets))
    ;[1 1 1] Primary Fire - Bullet
    (Game|SpawnActorfromClass "/Game/Blueprints/Combat/Bullet.Bullet_C" (Math|Transform|MakeTransform (Math|Transform|TransformLocation _returnvalue (Math|Vector|MakeVector 1e+02 0.0 0.0)) (Math|Rotator|CombineRotators (Math|Rotator|MakeRotator 0.0 (* (Math|Random|RandomFloatinRange -1.0 1.0) _accuracy) (* (Math|Random|RandomFloatinRange -1.0 1.0) _accuracy)) _rotation) _scale) "Undefined" 0 0)))