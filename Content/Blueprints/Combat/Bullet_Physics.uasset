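; Physics-driven bullet projectile that damages flying pawns it strikes.
; On BeginPlay it launches its static mesh with a fixed impulse along the mesh's forward direction, leaving movement to physics simulation.
; Hits on a FlyingPawn pass Damage to that pawn and decrement Penetration, destroying the bullet once it runs out; other hits only print debug text.
; Mesh overlaps only print a debug message.
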(event OnComponentHit(StaticMesh)
  (params (HitComponent :type Primitive%20Component%20Object%20Reference) (OtherActor :type Actor%20Object%20Reference) (OtherComp :type Primitive%20Component%20Object%20Reference) (NormalImpulse :type Vector :default "0, 0, 0") (Hit :type Hit%20Result%20Structure%20%28by%20ref%29))
  (bind _penetration (Variables|Default|GetPenetration))
  (Development|PrintString "Hit")
  (bind _asflying_pawn (Utilities|Casting|CastToFlyingPawn OtherActor))
  (Default|Damage _asflying_pawn (Variables|Default|GetDamage))
  (Math|Integer|DecrementInt _penetration
    (:%20%20
      (if (<= _penetration 0)
        (Actor|DestroyActor)))))

(event OnComponentBeginOverlap(StaticMesh)
  (params (OverlappedComponent :type Primitive%20Component%20Object%20Reference) (OtherActor :type Actor%20Object%20Reference) (OtherComp :type Primitive%20Component%20Object%20Reference) (OtherBodyIndex :type Integer) (bFromSweep :type Boolean) (SweepResult :type Hit%20Result%20Structure%20%28by%20ref%29))
  (Development|PrintString "Overlap"))

(event EventBeginPlay
  (Physics|AddImpulse (Variables|Default|GetStaticMesh) (Math|Vector|RotateVector (Math|Vector|MakeVector 2e+02 0.0 0.0) (Transformation|GetWorldRotation (Variables|Default|GetStaticMesh))) "None" false))

(event Collision|EventActorBeginOverlap
  (params (OtherActor :type Actor%20Object%20Reference)))

(event EventTick
  (params (DeltaSeconds :type Float%20%28single-precision%29)))

(fn ConstructionScript)