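; Rocket projectile actor that explodes when its collision component hits something, then destroys itself.
; On hit it spawns an Explosion actor scaled from ExplosionSize and runs a multi-sphere trace using that same value as radius, with timed debug drawing.
; Actors returned by the trace are destroyed outright, a placeholder until a damage script replaces it.
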(event OnComponentHit(CollisionComponent)
  (params (HitComponent :type Primitive%20Component%20Object%20Reference) (OtherActor :type Actor%20Object%20Reference) (OtherComp :type Primitive%20Component%20Object%20Reference) (NormalImpulse :type Vector :default "0, 0, 0") (Hit :type Hit%20Result%20Structure%20%28by%20ref%29))
  (bind _self self)
  (bind _collisioncomponent (Variables|Default|GetCollisionComponent _self))
  (bind _returnvalue (Transformation|GetWorldLocation _collisioncomponent))
  (Game|SpawnActorfromClass "/Game/Blueprints/Combat/Explosion.Explosion_C" (Math|Transform|MakeTransform _returnvalue "0, 0, 0" (Math|Conversions|ToVector(Float) (/ (Variables|Default|GetExplosionSize) 5e+01))) "Undefined" 0 0)
  (bind _outhits (Collision|MultiSphereTraceByChannel _returnvalue (+ _returnvalue "0.100000, 0, 0") (Variables|Default|GetExplosionSize) "TraceTypeQuery4" false 0 "ForDuration" true "(R=1.000000,G=0.000000,B=0.000000,A=1.000000)" "(R=0.000000,G=1.000000,B=0.000000,A=1.000000)" 2.0))
  (for _array_element _outhits
    (Actor|DestroyActor (|HitElement _array_element)) ; Replace later with damage script
  )
  (Actor|DestroyActor))

(event EventBeginPlay)

(event Collision|EventActorBeginOverlap
  (params (OtherActor :type Actor%20Object%20Reference)))

(event EventTick
  (params (DeltaSeconds :type Float%20%28single-precision%29)))

(fn ConstructionScript)