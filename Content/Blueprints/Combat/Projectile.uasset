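; Combat projectile Blueprint with homing logic toward a target point, currently inactive: Tick only checks the Homing flag.
; The disconnected chain converts the target direction into local space, derives a rotation, then applies it and moves forward by Speed times delta time.
; RotatorLimiter clamps pitch and yaw to HomingRate, preserving sign and zeroing roll.
; The turn limit applies per call, unscaled by delta time.
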(event EventBeginPlay)

(event Collision|EventActorBeginOverlap
  (params (OtherActor :type Actor%20Object%20Reference)))

(event EventTick
  (params (DeltaSeconds :type Float%20%28single-precision%29))
  (if (Variables|Default|GetHoming)
    _))

(fn ConstructionScript)

(fn RotatorLimiter
  (params (AttemptedRotation :type Rotator))
  (bind (_roll _pitch _yaw) (Math|Rotator|BreakRotator AttemptedRotation))
  (Utilities|FlowControl|Sequence
    (:then_0
      ;[1 1 1] Limit rotator rate
      (if (> (Math|Float|Absolute(Float) _pitch) (Variables|Default|GetHomingRate)) ; Check if Pitch change is greater than the limit
        (Variables|Default|SetHomingRotatorPitch (* (Variables|Default|GetHomingRate) (/ _pitch (Math|Float|Absolute(Float) _pitch)))) ; Set the Pitch change to the homing rate with correct sign
        (else
          (Variables|Default|SetHomingRotatorPitch _pitch))))
    (:then_1
      (if (> (Math|Float|Absolute(Float) _yaw) (Variables|Default|GetHomingRate)) ; Check if  Yaw change is greater than the limit
        (Variables|Default|SetHomingRotatorYaw (* (Variables|Default|GetHomingRate) (/ _yaw (Math|Float|Absolute(Float) _yaw)))) ; Set the Yaw change to the homing rate with correct sign
        (else
          (Variables|Default|SetHomingRotatorYaw _yaw)))
      (return (Math|Rotator|MakeRotator 0.0 (Variables|Default|GetHomingRotatorPitch) (Variables|Default|GetHomingRotatorYaw))))))