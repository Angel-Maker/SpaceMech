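; Weapon Blueprint that fires Bullet actors on behalf of whichever actor calls its Shoot event.
; Shoot checks a CanShoot flag, spawns a bullet, then holds the flag off for ShotCooldown seconds with a Delay to limit fire rate.
; SpawnBullet places the bullet 100 units along the shooter's local X axis, copying that actor's rotation and scale.
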(event Custom|Shoot
  (params (SpawningActor :type Actor%20Object%20Reference))
  (if (Variables|Default|GetCanShoot)
    (CallFunction|SpawnBullet SpawningActor)
    (Variables|Default|SetCanShoot false)
    (Utilities|FlowControl|Delay (Variables|Default|GetShotCooldown))
    (Variables|Default|SetCanShoot true)))

(event EventBeginPlay)

(event EventTick
  (params (DeltaSeconds :type Float%20%28single-precision%29)))

(fn SpawnBullet
  (params (SpawningActor :type Actor%20Object%20Reference))
  (bind _returnvalue (Transformation|GetActorTransform SpawningActor))
  (bind (_location _rotation _scale) (Math|Transform|BreakTransform _returnvalue))
  ;[1 1 1] Primary Fire - Bullet
  (Game|SpawnActorfromClass "/Game/Blueprints/Combat/Bullet.Bullet_C" (Math|Transform|MakeTransform (Math|Transform|TransformLocation _returnvalue "100.000000, 0, 0") _rotation _scale) "Undefined" 0 0))